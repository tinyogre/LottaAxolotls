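; BP_Marshmallow is a pickup that axolotl pawns eat to grow larger.
; Its static mesh reacts to both hit and overlap events, ignoring the axolotl player character and responding only to BP_AxolotlPawn actors.
; GetEaten destroys the marshmallow and multiplies the eating pawn's root component world scale, so each one compounds its size by ten percent.
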(event OnComponentHit(StaticMesh)
  (params (HitComponent :type Primitive%20Component%20Object%20Reference) (OtherActor :type Actor%20Object%20Reference) (OtherComp :type Primitive%20Component%20Object%20Reference) (NormalImpulse :type Vector :default "0, 0, 0") (Hit :type Hit%20Result%20Structure%20%28by%20ref%29))
  (Utilities|Casting|CastToBP_AxolotlPlayerCharacter OtherActor
    (:CastFailed
      (bind _asbp_axolotl_pawn (Utilities|Casting|CastToBP_AxolotlPawn OtherActor))
      (CallFunction|GetEaten _asbp_axolotl_pawn))))

(event OnComponentBeginOverlap(StaticMesh)
  (params (OverlappedComponent :type Primitive%20Component%20Object%20Reference) (OtherActor :type Actor%20Object%20Reference) (OtherComp :type Primitive%20Component%20Object%20Reference) (OtherBodyIndex :type Integer) (bFromSweep :type Boolean) (SweepResult :type Hit%20Result%20Structure%20%28by%20ref%29))
  (Utilities|Casting|CastToBP_AxolotlPlayerCharacter OtherActor
    (:CastFailed
      (bind _asbp_axolotl_pawn (Utilities|Casting|CastToBP_AxolotlPawn OtherActor))
      (CallFunction|GetEaten _asbp_axolotl_pawn))))

(event EventBeginPlay)

(event Collision|EventActorBeginOverlap
  (params (OtherActor :type Actor%20Object%20Reference)))

(event EventTick
  (params (DeltaSeconds :type Float%20%28single-precision%29)))

(fn ConstructionScript)

(fn GetEaten
  (params (By%20Axolotl :type BP%20Axolotl%20Pawn%20Object%20Reference))
  (bind _rootcomponent (Variables|/Script/Engine.Actor|GetRootComponent By%20Axolotl))
  (Actor|DestroyActor)
  (Transformation|SetWorldScale3D _rootcomponent (* (Transformation|GetWorldScale _rootcomponent) 1.1)))