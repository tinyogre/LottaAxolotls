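; BP_Rocket is a rocket that carries axolotl pawns upward and releases them at a maximum height.
; Pawns overlapping its sphere become hidden passengers, and their count is written to the game state's FollowerCount.
; Tick drops invalid passengers, integrates acceleration once Launch is called, and teleports riders along.
; Above MaxHeight it unhides and releases passengers there, then resets to its start location; level-switching code is unreachable.
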(event OnComponentBeginOverlap(Sphere)
  (params (OverlappedComponent :type Primitive%20Component%20Object%20Reference) (OtherActor :type Actor%20Object%20Reference) (OtherComp :type Primitive%20Component%20Object%20Reference) (OtherBodyIndex :type Integer) (bFromSweep :type Boolean) (SweepResult :type Hit%20Result%20Structure%20%28by%20ref%29))
  (bind _asbp_axolotl_pawn (Utilities|Casting|CastToBP_AxolotlPawn OtherActor))
  (Utilities|FlowControl|Sequence
    (:then_0
      (Utilities|Array|AddUnique (Variables|Default|GetPassengers) _asbp_axolotl_pawn))
    (:then_1
      (Rendering|SetActorHiddenInGame _asbp_axolotl_pawn true))
    (:then_2
      (Variables|/Game/Blueprints/BP_AxolotlPawn.BP_AxolotlPawn_C|SetOn%20Board%20Rocket _asbp_axolotl_pawn self))
    (:then_3
      (Variables|/Script/LottaAxolotls.LottaAxolotlsGameState|SetFollowerCount (.AsLotta%20Axolotls%20Game%20State (Utilities|Casting|CastToLottaAxolotlsGameState (Game|GetGameState))) (Utilities|Array|Length (Variables|Default|GetPassengers))))))

(event Custom|Launch
  (Variables|Default|SetIs%20Launched true))

(event Collision|EventActorBeginOverlap
  (params (OtherActor :type Actor%20Object%20Reference)))

(event EventTick
  (params (DeltaSeconds :type Float%20%28single-precision%29))
  (Utilities|FlowControl|Sequence
    (:then_0
      (CallFunction|ValidatePassengers))
    (:then_1
      (if (Variables|Default|GetIs%20Launched)
        (bind _output_get (Variables|Default|SetVelocity (+ (Variables|Default|GetVelocity) (* (Variables|Default|GetAcceleration) DeltaSeconds))))
        (Transformation|SetActorLocation (+ (Transformation|GetActorLocation) (* _output_get DeltaSeconds)) false false)
        (if (> (.z (Transformation|GetActorLocation)) (Variables|Default|GetMax%20Height))
          (for _array_element (Variables|Default|GetPassengers)
            (Rendering|SetActorHiddenInGame _array_element false)
            (Transformation|SetActorLocation _array_element (Transformation|GetActorLocation) false true)
            (Variables|/Game/Blueprints/BP_AxolotlPawn.BP_AxolotlPawn_C|SetOn%20Board%20Rocket _array_element 0))
          (CallFunction|Reset))))
    (:then_2
      (CallFunction|MovePassengerstoRocket))))

(event EventBeginPlay
  (Variables|Default|SetInitial%20Location (Transformation|GetActorLocation)))

(fn ConstructionScript)

(fn MovePassengerstoRocket
  (for _array_element (Variables|Default|GetPassengers)
    (Transformation|SetActorLocation _array_element (Transformation|GetActorLocation) false true)))

(fn Reset
  (Transformation|SetActorLocation (Variables|Default|GetInitial%20Location) false true)
  (Utilities|Array|Clear (Variables|Default|GetPassengers))
  (Variables|Default|SetVelocity "0, 0, 0")
  (Variables|Default|SetIs%20Launched false))

(fn ValidatePassengers
  (Utilities|Array|Clear (LocalVariables|GetNew%20Passengers))
  (for _array_element (Variables|Default|GetPassengers)
    (Utilities|IsValid _array_element
      (:Is%20Valid
        (Utilities|Array|Add (LocalVariables|GetNew%20Passengers) _array_element))))
  (Variables|Default|SetPassengers (LocalVariables|GetNew%20Passengers)))