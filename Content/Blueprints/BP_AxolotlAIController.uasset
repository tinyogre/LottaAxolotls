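; AI controller for axolotl pawns that follows the player on demand and otherwise wanders.
; BeginPlay caches the BP_AxolotlPlayerCharacter as Leader, and Tick steers straight toward it while its WantsToBeFollowed flag is set.
; Otherwise RandomMovement counts down a timer, picking a new random 3D direction and short random duration when it expires.
; Both modes use raw AddMovementInput, with no navmesh or behavior tree.
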(event EventBeginPlay
  (bind _returnvalue (Actor|GetActorOfClass "/Game/Blueprints/BP_AxolotlPlayerCharacter.BP_AxolotlPlayerCharacter_C"))
  (Variables|Default|SetLeader _returnvalue))

(event EventTick
  (params (DeltaSeconds :type Float%20%28single-precision%29))
  (bind _returnvalue (Pawn|GetControlledPawn))
  (bind _leader (Variables|Default|GetLeader))
  (if (Variables|/Game/Blueprints/BP_AxolotlPlayerCharacter.BP_AxolotlPlayerCharacter_C|GetWants%20To%20Be%20Followed _leader)
    (Pawn|Input|AddMovementInput _returnvalue (Math|Vector|Normalize (- (Transformation|GetActorLocation _leader) (Transformation|GetActorLocation _returnvalue))) 1.0 false)
    (else
      (CallFunction|RandomMovement DeltaSeconds))))

(fn ConstructionScript)

(fn RandomMovement
  (params (Delta%20Time :type Float%20%28double-precision%29))
  (Utilities|FlowControl|Sequence
    (:then_0
      (Variables|Default|SetRandom%20Duration (- (Variables|Default|GetRandom%20Duration) Delta%20Time))
      (if (<= (Variables|Default|GetRandom%20Duration) 0.0)
        (Variables|Default|SetRandom%20Duration (Math|Random|RandomFloatinRange 0.5 3.0))
        (Variables|Default|SetRandom%20Direction (Math|Random|RandomUnitVector))))
    (:then_1
      (Pawn|Input|AddMovementInput (Pawn|GetControlledPawn) (Variables|Default|GetRandom%20Direction) 1.0 false))))