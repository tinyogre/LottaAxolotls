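; BP_AxolotlBot is an axolotl bot pawn with customizable body and fringe colors.
; Its construction script creates dynamic material instances on the first two material slots of the Axolotl component.
; BodyColor and FringeColor feed the Color parameter of those two materials respectively.
; On BeginPlay it spawns its default controller, with no other gameplay logic in this graph.
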(event EventBeginPlay
  (Pawn|SpawnDefaultController))

(event Collision|EventActorBeginOverlap
  (params (OtherActor :type Actor%20Object%20Reference)))

(event EventTick
  (params (DeltaSeconds :type Float%20%28single-precision%29)))

(fn ConstructionScript
  (bind _axolotl (Variables|Default|GetAxolotl))
  (Utilities|FlowControl|Sequence
    (:then_0
      (bind _returnvalue (Rendering|Material|CreateDynamicMaterialInstance (Variables|Default|GetAxolotl) 0 (Rendering|Material|GetMaterial _axolotl 0) "None" :!class /Script/Engine.PrimitiveComponent))
      (Rendering|Material|SetVectorParameterValue _returnvalue "Color" (Variables|Default|GetBody%20Color) :!class /Script/Engine.MaterialInstanceDynamic))
    (:then_1
      (bind _returnvalue_2 (Rendering|Material|CreateDynamicMaterialInstance (Variables|Default|GetAxolotl) 1 (Rendering|Material|GetMaterial _axolotl 1) "None" :!class /Script/Engine.PrimitiveComponent))
      (Rendering|Material|SetVectorParameterValue _returnvalue_2 "Color" (Variables|Default|GetFringe%20Color) :!class /Script/Engine.MaterialInstanceDynamic))))